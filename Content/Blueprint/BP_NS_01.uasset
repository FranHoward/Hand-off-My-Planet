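; BP_NS_01 is a projectile-style actor that flies forward with an attached Niagara effect and spawns an impact effect on collision.
; Tick moves it at constant speed with a swept location update, without a movement component.
; The Sphere's first hit, guarded by IsHit, zeroes the Niagara Scale variable and spawns NS_01 just off the surface along the impact normal.
; The actor destroys itself after a short delay.
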(event OnComponentHit(Sphere)
  (params (HitComponent :type Primitive%20Component%20Object%20Reference) (OtherActor :type Actor%20Object%20Reference) (OtherComp :type Primitive%20Component%20Object%20Reference) (NormalImpulse :type Vector :default "0, 0, 0") (Hit :type Hit%20Result%20Structure%20%28by%20ref%29))
  (bind (_bblockinghit _binitialoverlap _time _distance _location _impactpoint _normal _impactnormal) (Collision|BreakHitResult Hit))
  (if (not (Variables|Default|GetIsHit))
    (Variables|Default|SetIsHit true)
    (Niagara|SetNiagaraVariable(Float) (Variables|Default|GetNiagara) "Scale" 0.0)
    (Niagara|SpawnSystematLocation "/Game/Niagara/Fireball/NS_01.NS_01" (+ _impactpoint (* _impactnormal 1.0)))
    (Utilities|FlowControl|Delay 1.0)
    (Actor|DestroyActor)))

(event EventBeginPlay)

(event Collision|EventActorBeginOverlap
  (params (OtherActor :type Actor%20Object%20Reference)))

(event EventTick
  (params (DeltaSeconds :type Float%20%28single-precision%29))
  (Transformation|SetActorLocation (+ (Transformation|GetActorLocation) (* (Transformation|GetActorForwardVector) (* DeltaSeconds 1e+03))) true false))

(fn ConstructionScript)