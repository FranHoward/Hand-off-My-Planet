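; BP_Gun is a gun actor that projects a continuous Niagara beam from its muzzle.
; It activates the Niagara component on BeginPlay, then line traces every Tick on the Visibility channel along the muzzle's forward vector for the beam's length.
; The beam start and end are fed to Niagara user parameters, with the end clipped to the impact point on a blocking hit.
; The file applies no damage or other hit response.
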(event EventBeginPlay
  (Components|Activation|Activate (Variables|Default|GetNiagara) false))

(event Collision|EventActorBeginOverlap
  (params (OtherActor :type Actor%20Object%20Reference)))

(event EventTick
  (params (DeltaSeconds :type Float%20%28single-precision%29))
  (bind _muzzle (Variables|Default|GetMuzzle))
  (bind _beamlength (Variables|Default|GetBeamLength))
  (bind _returnvalue (Transformation|GetWorldLocation _muzzle))
  (bind _returnvalue_2 (Math|Vector|GetForwardVector _muzzle))
  (bind _returnvalue_3 (* _returnvalue_2 _beamlength))
  (bind _returnvalue_4 (+ _returnvalue _returnvalue_3))
  (bind _outhit (Collision|LineTraceByChannel _returnvalue _returnvalue_4 "TraceTypeQuery1" false 0 "None"))
  (Niagara|SetNiagaraVariable(Vector3) (Variables|Default|GetNiagara) "User.BeamStart" _returnvalue)
  (Niagara|SetNiagaraVariable(Vector3) (Variables|Default|GetNiagara) "User.BeamEnd" (Math|Vector|SelectVector (.ImpactPoint (Collision|BreakHitResult _outhit)) _returnvalue_4 (.bBlockingHit (Collision|BreakHitResult _outhit)))))

(fn ConstructionScript)